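; Enemy spawner that creates BP_Enemy actors while the third-person player character is inside its SpawnArea.
; Entering starts a looping 0.8-second timer for SpawnEnemy, and leaving clears it.
; Each tick checks that a random reachable navmesh point around the spawner is not too near the player, then spawns with a 2D sound cue.
; The spawn location is a separate random query, so it can differ from the checked point.
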(event OnComponentBeginOverlap(SpawnArea)
  (params (OverlappedComponent :type Primitive%20Component%20Object%20Reference) (OtherActor :type Actor%20Object%20Reference) (OtherComp :type Primitive%20Component%20Object%20Reference) (OtherBodyIndex :type Integer) (bFromSweep :type Boolean) (SweepResult :type Hit%20Result%20Structure%20%28by%20ref%29))
  (bind _asbp_third_person_character (Utilities|Casting|CastToBP_ThirdPersonCharacter OtherActor))
  (Variables|Default|SetAs%20BP%20Third%20Person%20Character _asbp_third_person_character)
  (bind _returnvalue (Utilities|Time|SetTimerbyEvent (delegate Custom|SpawnEnemy) 0.8 true))
  (bind _output_get (Variables|Default|SetSpawnTimerHandle _returnvalue)))

(event OnComponentEndOverlap(SpawnArea)
  (params (OverlappedComponent :type Primitive%20Component%20Object%20Reference) (OtherActor :type Actor%20Object%20Reference) (OtherComp :type Primitive%20Component%20Object%20Reference) (OtherBodyIndex :type Integer))
  (bind _asbp_third_person_character (Utilities|Casting|CastToBP_ThirdPersonCharacter OtherActor))
  (Variables|Default|SetAs%20BP%20Third%20Person%20Character _asbp_third_person_character)
  (Utilities|Time|ClearandInvalidateTimerbyHandle (stale OnComponentBeginOverlap(SpawnArea) _output_get)))

(event Custom|SpawnEnemy
  (bind _returnvalue (Transformation|GetActorLocation))
  (bind _randomlocation (AI|Navigation|GetRandomReachablePointinRadius _returnvalue 1e+04 0 0))
  (if (>= (Math|Vector|Distance(Vector) _randomlocation (Transformation|GetActorLocation (Variables|Default|GetAs%20BP%20Third%20Person%20Character))) 2e+02)
    (Game|SpawnActorfromClass "/Game/AI/BP_Enemy.BP_Enemy_C" (Math|Transform|MakeTransform _randomlocation "0, 0, 0" "1.000000,1.000000,1.000000") "AlwaysSpawn" "MultiplyWithRoot" 0 0)
    (Audio|PlaySound2D "/Engine/EditorSounds/GamePreview/StartSimulate_Cue.StartSimulate_Cue" 1.0 1.0 0.0 0 0)))

(fn ConstructionScript)