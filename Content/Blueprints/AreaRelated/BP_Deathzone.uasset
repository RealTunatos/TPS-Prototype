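; BP_Deathzone is a trigger volume that ends the game when the player character enters it.
; On Death component overlap with BP_ThirdPersonCharacter, it sets the character's IsGameOver flag and disables its movement.
; It then switches to UI-only input with a visible cursor, shows the WBP_GameOver widget and freezes the world by setting global time dilation to zero.
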(event OnComponentBeginOverlap(Death)
  (params (OverlappedComponent :type Primitive%20Component%20Object%20Reference) (OtherActor :type Actor%20Object%20Reference) (OtherComp :type Primitive%20Component%20Object%20Reference) (OtherBodyIndex :type Integer) (bFromSweep :type Boolean) (SweepResult :type Hit%20Result%20Structure%20%28by%20ref%29))
  (bind _asbp_third_person_character (Utilities|Casting|CastToBP_ThirdPersonCharacter OtherActor))
  (Variables|/Game/ThirdPerson/Blueprints/BP_ThirdPersonCharacter.BP_ThirdPersonCharacter_C|SetIsGameOver _asbp_third_person_character true)
  (Pawn|Components|CharacterMovement|SetMovementMode (Variables|/Script/Engine.Character|GetCharacterMovement _asbp_third_person_character) "MOVE_None" 0)
  (Input|SetInputModeUIOnly (Game|GetPlayerController 0) 0 "DoNotLock" false)
  (Variables|/Script/Engine.PlayerController|SetbShowMouseCursor (Game|GetPlayerController 0) true)
  (bind _returnvalue (UserInterface|CreateWidget "/Game/Blueprints/Widgets/Other/WBP_GameOver.WBP_GameOver_C"))
  (UserInterface|Viewport|AddtoViewport _returnvalue 0)
  (Utilities|Time|SetGlobalTimeDilation 0.0))

(fn ConstructionScript)